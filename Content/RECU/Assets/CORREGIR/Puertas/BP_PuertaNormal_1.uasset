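; Door actor that swings a grille door (DOORrEJA) open while an actor tagged Player is inside its Box trigger.
; Box overlap begin and end drive a short eased MoveComponentTo that keeps the relative location and rotates the door open or back to zero rotation.
; Door collision is disabled as soon as opening starts and restored as soon as closing starts, without waiting for either move to finish.
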(event OnComponentBeginOverlap(Box)
  (params (OverlappedComponent :type Primitive%20Component%20Object%20Reference) (OtherActor :type Actor%20Object%20Reference) (OtherComp :type Primitive%20Component%20Object%20Reference) (OtherBodyIndex :type Integer) (bFromSweep :type Boolean) (SweepResult :type Hit%20Result%20Structure%20%28by%20ref%29))
  (bind _doorreja (Variables|Default|GetdOORrEJA))
  (if (Actor|ActorHasTag OtherActor "Player")
    (Components|MoveComponentTo _doorreja (Variables|/Script/Engine.SceneComponent|GetRelativeLocation _doorreja) "0.000000,120.000000,0.000000" false true 0.5 false)
    (Collision|SetCollisionEnabled _doorreja "NoCollision")))

(event OnComponentEndOverlap(Box)
  (params (OverlappedComponent :type Primitive%20Component%20Object%20Reference) (OtherActor :type Actor%20Object%20Reference) (OtherComp :type Primitive%20Component%20Object%20Reference) (OtherBodyIndex :type Integer))
  (bind _doorreja (Variables|Default|GetdOORrEJA))
  (if (Actor|ActorHasTag OtherActor "Player")
    (Components|MoveComponentTo _doorreja (Variables|/Script/Engine.SceneComponent|GetRelativeLocation _doorreja) "0, 0, 0" false true 0.5 false)
    (Collision|SetCollisionEnabled _doorreja "QueryAndPhysics")))

(event EventBeginPlay)

(event Collision|EventActorBeginOverlap
  (params (OtherActor :type Actor%20Object%20Reference)))

(event EventTick
  (params (DeltaSeconds :type Float%20%28single-precision%29)))

(fn ConstructionScript)