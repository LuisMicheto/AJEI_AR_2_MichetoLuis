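; BP_TERCERAPuerta is a door ("third door") that wins the game when its trigger box is overlapped while unlocked.
; An overlap with Unlocked set plays the unlock sound, waits briefly, plays a door squeak, then calls Win on MyHUD.
; Otherwise it calls DontHaveKey on the HUD.
; The overlap does not filter the overlapping actor, and Unlocked is only read here, never set.
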(event OnComponentBeginOverlap(Box)
  (params (OverlappedComponent :type Primitive%20Component%20Object%20Reference) (OtherActor :type Actor%20Object%20Reference) (OtherComp :type Primitive%20Component%20Object%20Reference) (OtherBodyIndex :type Integer) (bFromSweep :type Boolean) (SweepResult :type Hit%20Result%20Structure%20%28by%20ref%29))
  (bind _returnvalue (Game|GetPlayerController 0))
  (bind _returnvalue_2 (HUD|GetHUD _returnvalue))
  (if (Variables|Default|GetUnlocked)
    (Audio|PlaySound2D "/Game/RECU/Assets/Descargados/Unlock.Unlock" 1.0 1.0 0.0 0 0)
    (Utilities|FlowControl|Delay 0.2)
    (Audio|PlaySound2D "/Game/RECU/Assets/Descargados/Door_squeek.Door_squeek" 1.0 1.0 0.0 0 0)
    (bind _asmy_hud (Utilities|Casting|CastToMyHUD _returnvalue_2))
    (Default|Win _asmy_hud)
    (else
      (bind _asmy_hud_2 (Utilities|Casting|CastToMyHUD _returnvalue_2))
      (Default|DontHaveKey _asmy_hud_2))))

(event EventBeginPlay)

(event Collision|EventActorBeginOverlap
  (params (OtherActor :type Actor%20Object%20Reference)))

(event EventTick
  (params (DeltaSeconds :type Float%20%28single-precision%29)))

(fn ConstructionScript)