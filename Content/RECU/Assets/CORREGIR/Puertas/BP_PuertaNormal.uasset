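; BP_PuertaNormal is an automatic door that swings open when an actor tagged Player enters its Box trigger and closes when that actor leaves.
; Each swing plays a squeak sound and uses MoveComponentTo to rotate LaPuerta's yaw 120 degrees relative to its current rotation over half a second.
; Two DoOnce gates reset each other so opening and closing alternate, keeping the relative rotations from stacking.
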(event OnComponentBeginOverlap(Box)
  (params (OverlappedComponent :type Primitive%20Component%20Object%20Reference) (OtherActor :type Actor%20Object%20Reference) (OtherComp :type Primitive%20Component%20Object%20Reference) (OtherBodyIndex :type Integer) (bFromSweep :type Boolean) (SweepResult :type Hit%20Result%20Structure%20%28by%20ref%29))
  (bind _lapuerta (Variables|Default|GetLaPuerta))
  (bind _lapuerta_2 (Variables|Default|GetLaPuerta))
  (bind _relativerotation (Variables|/Script/Engine.SceneComponent|GetRelativeRotation _lapuerta))
  (bind _relativerotation_2 (Variables|/Script/Engine.SceneComponent|GetRelativeRotation _lapuerta_2))
  (if (Actor|ActorHasTag OtherActor "Player")
    (Utilities|FlowControl|DoOnce false
      (:Completed
        (Audio|PlaySound2D "/Game/RECU/Assets/Descargados/Door_squeek.Door_squeek" 1.0 1.0 0.0 0 0)
        (Components|MoveComponentTo _lapuerta_2 (Variables|/Script/Engine.SceneComponent|GetRelativeLocation _lapuerta_2) (Math|Rotator|MakeRotator (.roll _relativerotation_2) (.pitch _relativerotation_2) (+ (.yaw _relativerotation_2) -1.2e+02)) false false 0.5 false)
        (Utilities|FlowControl|DoOnce false) ; enters at Reset
      ))))

(event OnComponentEndOverlap(Box)
  (params (OverlappedComponent :type Primitive%20Component%20Object%20Reference) (OtherActor :type Actor%20Object%20Reference) (OtherComp :type Primitive%20Component%20Object%20Reference) (OtherBodyIndex :type Integer))
  (bind _lapuerta (Variables|Default|GetLaPuerta))
  (bind _lapuerta_2 (Variables|Default|GetLaPuerta))
  (bind _relativerotation (Variables|/Script/Engine.SceneComponent|GetRelativeRotation _lapuerta))
  (bind _relativerotation_2 (Variables|/Script/Engine.SceneComponent|GetRelativeRotation _lapuerta_2))
  (if (Actor|ActorHasTag OtherActor "Player")
    (Utilities|FlowControl|DoOnce false
      (:Completed
        (Audio|PlaySound2D "/Game/RECU/Assets/Descargados/Door_squeek.Door_squeek" 1.0 1.0 0.0 0 0)
        (Components|MoveComponentTo _lapuerta (Variables|/Script/Engine.SceneComponent|GetRelativeLocation _lapuerta) (Math|Rotator|MakeRotator (.roll _relativerotation) (.pitch _relativerotation) (- (.yaw _relativerotation) -1.2e+02)) false true 0.5 true)
        (Utilities|FlowControl|DoOnce false) ; enters at Reset
      ))))

(event EventBeginPlay)

(event Collision|EventActorBeginOverlap
  (params (OtherActor :type Actor%20Object%20Reference)))

(event EventTick
  (params (DeltaSeconds :type Float%20%28single-precision%29)))

(fn ConstructionScript)