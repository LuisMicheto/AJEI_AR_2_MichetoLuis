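; BP_Zombie is an enemy zombie character that spots, attacks and dies to the player.
; PawnSensing sets a blackboard flag and raises chase speed, while Passive drops it to a shamble.
; AttackPlayer stops movement and uses a montage notify for a sphere-overlap melee hit; point damage drains Health, triggering hit reactions or death and destruction.
; Tick repeatedly calls ZombieRoar, whose random Delay spaces out the 2D roar sounds.
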(event OnSeePawn(PawnSensing)
  (params (Pawn :type Pawn%20Object%20Reference))
  (if (not (Variables|Default|GetIsDead?))
    (AI|Components|Blackboard|SetValueasBool (AI|GetBlackboard 0) (Utilities|Name|MakeLiteralName "Can see Player?") true)
    (Variables|/Script/Engine.CharacterMovementComponent|SetMaxWalkSpeed (Variables|Character|GetCharacterMovement) 3.5e+02)))

(event Custom|ZombieRoar
  (Utilities|FlowControl|Delay (Math|Random|RandomFloatinRange 3.0 9.0))
  (Audio|PlaySound2D "/Game/RECU/Assets/Descargados/Zombies.Zombies" 1.0 1.0 0.0 0 0))

(event Custom|AttackPlayer
  (Variables|/Script/Engine.CharacterMovementComponent|SetMaxWalkSpeed (Variables|Character|GetCharacterMovement) 0.0)
  (Animation|Montage|PlayMontage (Variables|Character|GetMesh) "/Game/RECU/Assets/CORREGIR/Zombie/ZombieAnim/zombie_attack_Montage.zombie_attack_Montage"
    (:OnNotifyBegin
      (bind (_outactors _returnvalue) (Collision|SphereOverlapActors (Transformation|GetWorldLocation (Variables|Default|GetArrow1)) 8e+01 (Utilities|Array|MakeArray "ObjectTypeQuery3") "/Game/RECU/Assets/CORREGIR/Blueprints/BP_FirstPersonMINE.BP_FirstPersonMINE_C" (Utilities|Array|MakeArray self)))
      (if _returnvalue
        (for _array_element _outactors
          (Game|Damage|ApplyDamage _array_element 2e+01 (Pawn|GetController) self "/Script/Engine.DamageType")
          (Variables|/Script/Engine.CharacterMovementComponent|SetMaxWalkSpeed (Variables|Character|GetCharacterMovement) 3.5e+02))))))

(event Custom|Death
  (Variables|Default|SetIsDead? true)
  (Components|Movement|StopMovementImmediately (Variables|Character|GetCharacterMovement))
  (Animation|Montage|PlayMontage (Variables|Character|GetMesh) "/Game/RECU/Assets/CORREGIR/Zombie/ZombieAnim/zombie_dying_Montage.zombie_dying_Montage"
    (:then
      (Collision|SetCollisionResponsetoChannel (Variables|Collision|GetCapsuleComponent) "ECC_Pawn" "ECR_Overlap")
      (Collision|SetCollisionEnabled (Variables|Character|GetMesh) "NoCollision"))
    (:OnCompleted
      (Utilities|FlowControl|Delay 2.0)
      (Actor|DestroyActor))))

(event Custom|Passive
  (Variables|/Script/Engine.CharacterMovementComponent|SetMaxWalkSpeed (Variables|Character|GetCharacterMovement) 6e+01))

(event EventBeginPlay)

(event Collision|EventActorBeginOverlap
  (params (OtherActor :type Actor%20Object%20Reference)))

(event Game|Damage|EventPointDamage
  (params (Damage :type Float%20%28single-precision%29) (DamageType :type Damage%20Type%20Object%20Reference) (HitLocation :type Vector :default "0, 0, 0") (HitNormal :type Vector :default "0, 0, 0") (HitComponent :type Primitive%20Component%20Object%20Reference) (BoneName :type Name :default "None") (ShotFromDirection :type Vector :default "0, 0, 0") (InstigatedBy :type Controller%20Object%20Reference) (DamageCauser :type Actor%20Object%20Reference) (HitInfo :type Hit%20Result%20Structure%20%28by%20ref%29))
  (if (not (Variables|Default|GetIsDead?))
    (if (<= (Variables|Default|GetHealth) 0.0)
      (CallFunction|Death)
      (else
        (bind _output_get (Variables|Default|SetHealth (- (Variables|Default|GetHealth) Damage)))
        (if (<= _output_get 0.0)
          (CallFunction|Death)
          (else
            (Animation|Montage|PlayMontage (Variables|Character|GetMesh) "/Game/RECU/Assets/CORREGIR/Zombie/ZombieAnim/Zombie_Reaction_Hit_mixamo_com_Montage.Zombie_Reaction_Hit_mixamo_com_Montage")))))))

(event EventTick
  (params (DeltaSeconds :type Float%20%28single-precision%29))
  (CallFunction|ZombieRoar))

(fn ConstructionScript)